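; Light receiver block that serves as the goal, ending the game when light reaches it.
; Binds to the light-reached event and, once only, asks MyGGJ2018GameModeBase to show the end screen.
; The construction script tints the mesh and crystal with a dynamic material instance matching the target light's colour.
; Tick spins the crystal by a fixed step each frame, independent of delta time.
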(event Custom|EndGame
  (Utilities|FlowControl|DoOnce false
    (:Completed
      (bind _asmy_ggj2018game_mode_base (Utilities|Casting|CastToMyGGJ2018GameModeBase (Game|GetGameMode)))
      (Default|ShowGameEndScreen _asmy_ggj2018game_mode_base))))

(event EventBeginPlay
  (EventDispatchers|BindEventtoOnLightReachedPoint (delegate Custom|EndGame)))

(event Collision|EventActorBeginOverlap
  (params (OtherActor :type Actor%20Object%20Reference)))

(event EventTick
  (params (DeltaSeconds :type Float%20%28single-precision%29))
  (Transformation|AddLocalRotation (Variables|Default|GetCrystal) "0,1.000000, 0" false false))

(fn ConstructionScript
  (bind _returnvalue (Rendering|Material|CreateDynamicMaterialInstance "/Game/Models/Background_Seamless_texture_Mat.Background_Seamless_texture_Mat" :!class /Script/Engine.KismetMaterialLibrary))
  (Rendering|Material|SetVectorParameterValue _returnvalue "Colour" (Math|Conversions|ToLinearColor(Color) (Utilities|Struct|BreakLightInfo (Variables|Default|GetTargetLight))) :!class /Script/Engine.MaterialInstanceDynamic)
  (Rendering|Material|SetMaterial (Variables|Default|GetStaticMesh) 0 _returnvalue))